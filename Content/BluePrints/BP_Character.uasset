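; BP_Character is a character Blueprint that alternates between AI movement toward the player controller and standing still.
; Tick accumulates a wait timer and flips an IsMoving flag, starting AI MoveTo after a short pause and stopping movement immediately after a longer moving phase.
; The move targets the player controller actor rather than its pawn, and debug text prints on each start and stop.
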(event `self.ReceiveBeginPlay`)

(event `self.ReceiveTick`
  (params (DeltaSeconds :type "Float (single-precision)"))
  (set `self.WaitTime` (+ DeltaSeconds (`self.WaitTime`)))
  (if (`self.IsMoving`)
    (if (> (`self.WaitTime`) 5.0)
      (set `self.IsMoving` false)
      (set `self.WaitTime` 0.0)
      (`MovementComponent.StopMovementImmediately` (`self.CharacterMovement`))
      (`KismetSystemLibrary.PrintText` "Stop"))
    (elif (> (`self.WaitTime`) 3.0)
      (set `self.IsMoving` true)
      (set `self.WaitTime` 0.0)
      (`|AIMoveTo` self (0.0 0.0 0.0) (`GameplayStatics.GetPlayerController` 0)
        (:`then`
          (`KismetSystemLibrary.PrintText` "Go"))))))

(fn `UserConstructionScript`)