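; BP_Enemy is an enemy actor that tracks itself in the game instance's shared enemy list.
; On BeginPlay it casts the game instance to BP_GameInstance, stores it and adds itself to EnemyList.
; GetAttackByPlayer removes the enemy from that list and destroys it, so a single call kills it with no health logic.
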(event `self.ReceiveBeginPlay`
  (bind _asbp_game_instance (cast `/Game/BluePrints/BP_GameInstance` (`GameplayStatics.GetGameInstance`)))
  (bind _output_get (set `self.BP Game Instance` _asbp_game_instance))
  (`KismetArrayLibrary.Array_Add` (`/Game/BluePrints/BP_GameInstance.EnemyList` _output_get) self))

(fn `GetAttackByPlayer`
  (for _array_element (`/Game/BluePrints/BP_GameInstance.EnemyList` (`self.BP Game Instance`))
    (if (== _array_element self)
      (`KismetArrayLibrary.Array_RemoveItem` (`/Game/BluePrints/BP_GameInstance.EnemyList` (`self.BP Game Instance`)) _array_element)
      (break)))
  (`self.K2_DestroyActor`))

(fn `UserConstructionScript`)