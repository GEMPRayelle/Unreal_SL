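; Enemy spawn controller that periodically places BP_Enemy actors in the level, up to a small fixed count.
; Tick accumulates delta time into a cooldown and, once it exceeds the interval while the count is under the cap, spawns an enemy and resets the timer.
; Each spawn uses a random X/Y position in a square around the world origin at zero height.
; The counter only increases, so spawning stops permanently at the cap.
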(event `self.ReceiveBeginPlay`
  (set `self.SpawnCount` 0))

(event `self.ReceiveTick`
  (params (DeltaSeconds :type "Float (single-precision)"))
  (bind _output_get (set `self.CoolTime` (+ DeltaSeconds (`self.CoolTime`))))
  (if (> _output_get 2.0)
    (if (< (`self.SpawnCount`) 5)
      (`|SpawnActorFromClass` "/Game/BluePrints/BP_Enemy.BP_Enemy_C" (`KismetMathLibrary.MakeTransform` (`KismetMathLibrary.MakeVector` (`KismetMathLibrary.RandomFloatInRange` -800.0 800.0) (`KismetMathLibrary.RandomFloatInRange` -800.0 800.0))) "Undefined" "MultiplyWithRoot" null null)
      (set `self.CoolTime` 0.0)
      (`/Engine/EditorBlueprintResources/StandardMacros.IncrementInt` (`self.SpawnCount`)))))

(fn `UserConstructionScript`)